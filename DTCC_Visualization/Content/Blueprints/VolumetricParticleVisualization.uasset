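; Actor that visualizes volumetric data as Niagara particles, with wind speed scale, spawn and appearance settings.
; The construction script assigns the particle system, positions the component from a material parameter collection offset, then calls PropagateParameters.
; PropagateParameters feeds Niagara the collection's scale, rotation and half-extent-shifted XY offset, plus the actor's tuning variables.
; Reset sets KillParticles to its input, then clears it after a short delay.
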(event Custom|Reset
  (params (Param :type Boolean))
  (bind _niagaracomponent (Variables|NiagaraActor|GetNiagaraComponent))
  (Effects|Components|ParticleSystem|SetBoolParameter _niagaracomponent "KillParticles" Param)
  (Utilities|FlowControl|Delay 0.2)
  (Effects|Components|ParticleSystem|SetBoolParameter _niagaracomponent "KillParticles" false))

(event EventBeginPlay)

(event EventTick
  (params (DeltaSeconds :type Float%20%28single-precision%29)))

(fn ConstructionScript
  (Class|NiagaraComponent|SetAsset (Variables|NiagaraActor|GetNiagaraComponent) (Variables|Default|GetParticleSystem) true)
  (bind _returnvalue (Rendering|Material|GetVectorParameterValue "/DTCC_Visualization/ParameterCollections/VolumetricDataPositioningParameters.VolumetricDataPositioningParameters" "PositionOffset" :!class /Script/Engine.KismetMaterialLibrary))
  (Transformation|SetWorldLocation (Variables|NiagaraActor|GetNiagaraComponent) (Math|Conversions|ToVector(LinearColor) _returnvalue) false false)
  (CallFunction|PropagateParameters))

(fn PropagateParameters
  (bind _niagaracomponent (Variables|NiagaraActor|GetNiagaraComponent))
  (bind _niagaracomponent_2 (Variables|NiagaraActor|GetNiagaraComponent))
  (bind _volumetricdatapositioningparametercollection (Variables|Default|GetVolumetricDataPositioningParameterCollection))
  ;[1 1 1] Get from VolumetricDataPositionParameters parameter collection
  (bind _returnvalue (Rendering|Material|GetVectorParameterValue _volumetricdatapositioningparametercollection (Utilities|Name|MakeLiteralName "Scale") :!class /Script/Engine.KismetMaterialLibrary))
  (Effects|Components|ParticleSystem|SetVectorParameter (Variables|NiagaraActor|GetNiagaraComponent) "DataScale" (Math|Conversions|ToVector(LinearColor) _returnvalue))
  (bind _returnvalue_2 (Rendering|Material|GetVectorParameterValue _volumetricdatapositioningparametercollection (Utilities|Name|MakeLiteralName "PositionOffset") :!class /Script/Engine.KismetMaterialLibrary))
  (Effects|Components|ParticleSystem|SetVectorParameter (Variables|NiagaraActor|GetNiagaraComponent) "DataPositionOffset" (+ (Math|Conversions|ToVector(LinearColor) _returnvalue_2) (* (Math|Conversions|ToVector(LinearColor) _returnvalue) "-50.000000,-50.000000,0.000000")))
  (bind _returnvalue_3 (Rendering|Material|GetScalarParameterValue _volumetricdatapositioningparametercollection (Utilities|Name|MakeLiteralName "Rotation") :!class /Script/Engine.KismetMaterialLibrary))
  (Effects|Components|ParticleSystem|SetFloatParameter (Variables|NiagaraActor|GetNiagaraComponent) "DataRotation" _returnvalue_3)
  (Effects|Components|ParticleSystem|SetBoolParameter _niagaracomponent_2 "KillParticles" false)
  (Effects|Components|ParticleSystem|SetFloatParameter _niagaracomponent_2 "Opacity" (Variables|Default|GetOpacity))
  (Effects|Components|ParticleSystem|SetFloatParameter _niagaracomponent_2 "EmissiveGain" (Variables|Default|GetEmissiveGain))
  (Effects|Components|ParticleSystem|SetFloatParameter _niagaracomponent_2 "SpawnRate" (Variables|Default|GetSpawnRate))
  (Effects|Components|ParticleSystem|SetFloatParameter _niagaracomponent_2 "MaxLifetime" (Variables|Default|GetMaxLifetime))
  (Effects|Components|ParticleSystem|SetFloatParameter _niagaracomponent "MinSpriteSize" (Variables|Default|GetMinSpriteSize))
  (Effects|Components|ParticleSystem|SetFloatParameter _niagaracomponent "WindSpeedScale" (Variables|Default|GetWindSpeedScale))
  (Effects|Components|ParticleSystem|SetVectorParameter _niagaracomponent "DataSpawnCrop" (Variables|Default|GetDataSpawnCrop))
  (Effects|Components|ParticleSystem|SetVectorParameter _niagaracomponent "DataSpawnJustify" (Variables|Default|GetDataSpawnJustify)))