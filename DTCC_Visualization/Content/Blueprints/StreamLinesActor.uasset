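; Actor that visualizes a labeled streamline dataset from a data table as Niagara particle effects and static procedural meshes.
; Construction loads the dataset, builds Niagara components split by line count per enabled style, and assigns static lines to a cell-based segment generator.
; Materials combine high/low position textures into a 32-bit render target and bake velocity into another.
; Static Streamline actors spawn in delayed bursts, painted by velocity.
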(event Custom|TestNiagara
  (Utilities|IsValid (Utilities|Array|Get(acopy) (Variables|Default|GetStreamlineSystems))
    (:Is%20Valid
      (Utilities|FlowControl|FlipFlop))))

(event Custom|TestStatic
  (Class|StreamlineSegmentGenerator|DynamicStreamlineSpawn (Variables|Default|GetStreamlineSegmentGenerator)))

(event EventBeginPlay
  (bind _linedatatexturesource (Variables|Default|GetLineDataTextureSource))
  (bind (_linetype _label _sourcepath _numlines _positionmin _positionmax _datamin _datamax _positiontexture _texturecombininglodivider _positiontexture_lo) (Utilities|Struct|BreakLineDataTextureSource _linedatatexturesource))
  (Utilities|FlowControl|Sequence
    (:then_0
      (if (Variables|Default|GetEnableParticleStreamlines)
        (CallFunction|PrepareDataTexture)
        (bind _output_get (Variables|/Script/Engine.Texture|SetMipLoadOptions _positiontexture "OnlyFirstMip"))
        (Variables|/Script/Engine.Texture|SetMipLoadOptions _positiontexture_lo _output_get)))
    (:then_1
      (if (Variables|Default|GetEnableStaticStreamlines)
        (CallFunction|SpawnStreamlines)))))

(event EventTick
  (params (DeltaSeconds :type Float%20%28single-precision%29)))

(event Custom|SpawnStreamlinesBurst
  (bind _numberofstreamlines (Variables|Default|GetNumberOfStreamLines))
  (bind _linedatatexturesource (Variables|Default|GetLineDataTextureSource))
  (bind _datarownames (Variables|Default|GetDataRowNames))
  (bind (_linetype _label _sourcepath _numlines _positionmin _positionmax _datamin _datamax _positiontexture _texturecombininglodivider _positiontexture_lo _datatexture _velocityspeedmin _velocityspeedmax) (Utilities|Struct|BreakLineDataTextureSource _linedatatexturesource))
  (bind _returnvalue (Utilities|Array|Length _datarownames))
  (bind _returnvalue_2 (Math|Integer|Min(Integer) _returnvalue _numberofstreamlines))
  ;[1 1 1] Spawn Streamlines
  (if (< (Variables|Spawning|GetSpawningLastLine) _returnvalue_2)
    (for _index (range (Variables|Spawning|GetSpawningLastLine) (Math|Integer|Min(Integer) (+ (Variables|Spawning|GetSpawningLastLine) (Variables|Spawning|GetSpawningBurstCount)) (- _returnvalue_2 1)))
      (bind _returnvalue_3 (Utilities|GetDataTableRow (.DataTable (Utilities|Struct|BreakLineDataTextureSource (Variables|Default|GetLineDataTextureSource))) (Utilities|Array|Get(acopy) (Variables|Default|GetDataRowNames) _index))
        (:then
          (bind _returnvalue_4 (Class|Streamline|SpawnStreamline self (.StreamlineName (Utilities|Struct|BreakVCStreamline _returnvalue_3)) (.Points (Utilities|Struct|BreakVCStreamline _returnvalue_3)) (* (Variables|Default|GetLineWidth) 0.5) (Variables|Default|GetStaticStreamlinesCapVertices)))
          (Class|Streamline|PaintStreamline _returnvalue_4 _velocityspeedmin _velocityspeedmax false)
          (Rendering|Material|SetMaterial (Variables|/Script/StreamlinesPlugin.Streamline|GetVCProceduralMeshComponent _returnvalue_4) 0 (Variables|Default|GetStaticStreamlineMaterial))
          (Transformation|AttachComponentToComponent _returnvalue_4 (Variables|Default|GetStaticStreamlines) "None" "KeepRelative" "KeepRelative" "KeepRelative" true))))
    (Variables|Spawning|SetSpawningLastLine _index)
    (Utilities|FlowControl|Delay 0.01)
    (CallFunction|SpawnStreamlinesBurst)
    (else
      (Development|PrintString (Utilities|String|ToString(Text) (Utilities|Text|FormatText "Spawning Complete ({n} lines)" _returnvalue_2)) true true "(R=0.000000,G=0.660000,B=1.000000,A=1.000000)" 5.0))))

(event Custom|SpawnStreamlines
  ;[1 1 1] Spawn Streamlines
  (Variables|Spawning|SetSpawningLastLine 0)
  (bind _outrownames (DataTable|GetDataTableRowNames (.DataTable (Utilities|Struct|BreakLineDataTextureSource (Variables|Default|GetLineDataTextureSource)))))
  (Variables|Default|SetDataRowNames _outrownames)
  (CallFunction|SpawnStreamlinesBurst))

(fn ConstructionScript
  (CallFunction|LoadandApplyData))

(fn PrepareDataTexture
  (bind _linedatatexturesource (Variables|Default|GetLineDataTextureSource))
  (bind (_linetype _label _sourcepath _numlines _positionmin _positionmax _datamin _datamax _positiontexture _texturecombininglodivider _positiontexture_lo _datatexture) (Utilities|Struct|BreakLineDataTextureSource _linedatatexturesource))
  (Utilities|FlowControl|Sequence
    (:then_0
      (bind _returnvalue (Rendering|Material|CreateDynamicMaterialInstance "/DTCC_Visualization/Materials/DataTexture32BitCombiner_Mat_Mat.DataTexture32BitCombiner_Mat_Mat" "None" "None" :!class /Script/Engine.KismetMaterialLibrary))
      (Rendering|Material|SetTextureParameterValue _returnvalue "Low" _positiontexture_lo)
      (Rendering|Material|SetTextureParameterValue _returnvalue "High" _positiontexture)
      (Rendering|Material|SetScalarParameterValue _returnvalue "LowFactor" (Math|Float|SelectFloat 0.0 (/ 1.0 _texturecombininglodivider) (== _texturecombininglodivider 0.0)) :!class /Script/Engine.MaterialInstanceDynamic)
      (Rendering|DrawMaterialtoRenderTarget "/DTCC_Visualization/RenderTargets/StreamlinesData_RT.StreamlinesData_RT" _returnvalue)
      (Variables|Default|SetIsDataPrepared true)
      (Rendering|Material|SetMaterial (Variables|Default|GetDebug) 0 _returnvalue))
    (:then_1
      (bind _returnvalue_2 (Rendering|Material|CreateDynamicMaterialInstance "/DTCC_Visualization/Materials/DataTexture_BakingMat.DataTexture_BakingMat" "None" "None" :!class /Script/Engine.KismetMaterialLibrary))
      (Rendering|Material|SetTextureParameterValue _returnvalue_2 "DataTexture" _datatexture)
      (Rendering|DrawMaterialtoRenderTarget "/DTCC_Visualization/RenderTargets/StreamlinesVelocity_RT.StreamlinesVelocity_RT" _returnvalue_2)
      (Development|PrintString (Utilities|String|Append "Prepared streamlined: " _label " : " (Utilities|String|ToString(Float) (Utilities|Time|GetGameTimeinSeconds)))))))

(fn SetupStreamlinesComponent
  (params (NiagaraSystem :type Niagara%20Component%20Object%20Reference) (NumberOfLines :type Integer) (LinesOffset :type Integer))
  (bind _linedatatexturesource (Variables|Default|GetLineDataTextureSource))
  (bind (_linetype _label _sourcepath _numlines _positionmin _positionmax _datamin _datamax _positiontexture _texturecombininglodivider _positiontexture_lo _datatexture _velocityspeedmin _velocityspeedmax) (Utilities|Struct|BreakLineDataTextureSource _linedatatexturesource))
  (Effects|Components|ParticleSystem|SetIntParameter NiagaraSystem "LinesNumber" NumberOfLines)
  (Effects|Components|ParticleSystem|SetIntParameter NiagaraSystem "LinesStepping" (Variables|Default|GetLinesStepping))
  (Effects|Components|ParticleSystem|SetIntParameter NiagaraSystem "LinesOffset" LinesOffset)
  (Effects|Components|ParticleSystem|SetVectorParameter NiagaraSystem "MinPosition" (.OutConvertedVector (Math|Conversions|ToVector(Float) _positionmin)))
  (Effects|Components|ParticleSystem|SetVectorParameter NiagaraSystem "MaxPosition" (.OutConvertedVector (Math|Conversions|ToVector(Float) _positionmax)))
  (Effects|Components|ParticleSystem|SetVectorParameter NiagaraSystem "MinVelocity" (.OutConvertedVector (Math|Conversions|ToVector(Float) _datamin)))
  (Effects|Components|ParticleSystem|SetVectorParameter NiagaraSystem "MaxVelocity" (.OutConvertedVector (Math|Conversions|ToVector(Float) _datamax)))
  (Effects|Components|ParticleSystem|SetVectorParameter NiagaraSystem "AxisScaling" (Variables|Default|GetAxisScaling))
  (Effects|Components|ParticleSystem|SetFloatParameter NiagaraSystem "SpeedMin" _velocityspeedmin)
  (Effects|Components|ParticleSystem|SetFloatParameter NiagaraSystem "SpeedMax" _velocityspeedmax))

(fn PrepareData
  (LocalVariables|SetDatasetFound false)
  (bind _outrownames (DataTable|GetDataTableRowNames (Variables|Default|GetLineDataTable)))
  (bind _array_element (Utilities|Array|ForEachLoopwithBreak _outrownames :!label _label)
    (:LoopBody
      (bind _returnvalue (Utilities|GetDataTableRow (Variables|Default|GetLineDataTable) _array_element)
        (:then
          (if (and (Utilities|Name|Equal(Name) (.LineType (Utilities|Struct|BreakLineDataTextureSource _returnvalue)) "StreamLines") (Utilities|Enum|Equal(Enum) (.Label (Utilities|Struct|BreakLineDataTextureSource _returnvalue)) (Variables|Default|GetDataLabel)))
            (LocalVariables|SetDatasetFound true)
            (Variables|Default|SetLineDataTextureSource _returnvalue)
            (goto _label Break)))))
    (:Completed
      (if (LocalVariables|GetDatasetFound)
        (CallFunction|PrepareDataTexture)
        (bind _output_get (Variables|Default|SetMaxNumberOfLines (Math|Float|Truncate (* (.NumLines (Utilities|Struct|BreakLineDataTextureSource (Variables|Default|GetLineDataTextureSource))) (.LinesPerTextureRow (Utilities|Struct|BreakLineDataTextureSource (Variables|Default|GetLineDataTextureSource)))))))
        (Variables|Default|SetNumberOfStreamLines (Math|Integer|Min(Integer) _output_get (Variables|Default|GetNumberOfStreamLines)))
        (else
          (Development|PrintText (Utilities|Text|FormatText "Dataset {label} not found in table {table}" (Variables|Default|GetDataLabel) (Class|KismetSystemLibrary|GetPathName (Variables|Default|GetLineDataTable))) true true "(R=1.000000,G=0.604933,B=0.187166,A=1.000000)" 1e+01))))))

(fn StyleStreamlinesSystem
  (params (NiagaraSystem :type Niagara%20Component%20Object%20Reference))
  (Effects|Components|ParticleSystem|SetFloatParameter NiagaraSystem "SpawnRate" (* (Variables|Default|GetSpawnRatePerTextureLine) (Utilities|GetNumberOfTextureLines)))
  (Effects|Components|ParticleSystem|SetFloatParameter NiagaraSystem "ParticleSize" (Variables|Default|GetParticleSize))
  (Effects|Components|ParticleSystem|SetFloatParameter NiagaraSystem "LineWidth" (Variables|Default|GetLineWidth))
  (Effects|Components|ParticleSystem|SetFloatParameter NiagaraSystem "ColorCurveFactor" (Variables|Default|GetColorCurveFactor)))

(fn ApplyStreamlinesStyle
  (for _array_element (Variables|Default|GetStreamlineSystems)
    (CallFunction|StyleStreamlinesSystem _array_element)))

(fn SetupDebug
  (bind _linedatatexturesource (Variables|Default|GetLineDataTextureSource))
  (bind _particlestreamlines (Variables|Default|GetParticleStreamlines))
  (bind _showfeaturedebug (Variables|Features|GetShowFeatureDebug))
  (bind (_linetype _label _sourcepath _numlines _positionmin _positionmax) (Utilities|Struct|BreakLineDataTextureSource _linedatatexturesource))
  (bind _returnvalue (not _showfeaturedebug))
  (Utilities|FlowControl|Sequence
    (:then_0
      (bind _output_get (Variables|Default|SetDataPositionMin (* (.OutConvertedVector (Math|Conversions|ToVector(Float) _positionmin)) (Variables|Default|GetAxisScaling))))
      (bind _output_get_2 (Variables|Default|SetDataPositionMax (* (.OutConvertedVector (Math|Conversions|ToVector(Float) _positionmax)) (Variables|Default|GetAxisScaling))))
      (Transformation|SetRelativeLocation (Variables|Default|GetPosMaxMarker) (- _output_get_2 _output_get) false false)
      (if (Variables|Default|GetPositionInAbsoluteWorld)
        (Transformation|SetWorldLocation _particlestreamlines (Variables|Default|GetDataPositionMin) false false)
        (else
          (Transformation|SetRelativeLocation _particlestreamlines "0, 0, 0" false false))))
    (:then_1
      (Development|SetHiddeninGame (Variables|Default|GetDebug) _returnvalue false)
      (Development|SetHiddeninGame (Variables|Default|GetPosMinMarker) _returnvalue false)
      (Development|SetHiddeninGame (Variables|Default|GetPosMaxMarker) _returnvalue false))))

(fn InitateNiagraSystems
  (bind _streamlinesystems (Variables|Default|GetStreamlineSystems))
  (for _array_element _streamlinesystems
    (Components|DestroyComponent _array_element))
  (Utilities|Array|Clear _streamlinesystems)
  (for _index (range 0 (/ (- (Utilities|GetNumberOfTextureLines) 1) (Variables|Default|GetMaxLinesPerComponent)))
    (Utilities|FlowControl|Sequence
      (:then_0
        (if (Variables|Features|GetShowFeatureDebug)
          (CallFunction|AddNiagaraSystemComponent (Math|Integer|Min(Integer) (- (+ (Variables|Default|GetNumberOfStreamLines) (Variables|Default|GetLinesOffset)) (+ (* _index (Variables|Default|GetMaxLinesPerComponent)) (Variables|Default|GetLinesOffset))) (Variables|Default|GetMaxLinesPerComponent)) (+ (* _index (Variables|Default|GetMaxLinesPerComponent)) (Variables|Default|GetLinesOffset)) "/DTCC_Visualization/Niagara/StreamlinesParticleSystem_DebugInfo.StreamlinesParticleSystem_DebugInfo")))
      (:then_1
        (if (Variables|Features|GetShowFeatureSprites)
          (CallFunction|AddNiagaraSystemComponent (Math|Integer|Min(Integer) (- (+ (Variables|Default|GetNumberOfStreamLines) (Variables|Default|GetLinesOffset)) (+ (* _index (Variables|Default|GetMaxLinesPerComponent)) (Variables|Default|GetLinesOffset))) (Variables|Default|GetMaxLinesPerComponent)) (+ (* _index (Variables|Default|GetMaxLinesPerComponent)) (Variables|Default|GetLinesOffset)) "/DTCC_Visualization/Niagara/StreamlinesParticleSystem_Sprites.StreamlinesParticleSystem_Sprites")))
      (:then_2
        (if (Variables|Features|GetShowFeatureMovingSprites)
          (CallFunction|AddNiagaraSystemComponent (Math|Integer|Min(Integer) (- (+ (Variables|Default|GetNumberOfStreamLines) (Variables|Default|GetLinesOffset)) (+ (* _index (Variables|Default|GetMaxLinesPerComponent)) (Variables|Default|GetLinesOffset))) (Variables|Default|GetMaxLinesPerComponent)) (+ (* _index (Variables|Default|GetMaxLinesPerComponent)) (Variables|Default|GetLinesOffset)) "/DTCC_Visualization/Niagara/StreamlinesParticleSystem_MovingSprites.StreamlinesParticleSystem_MovingSprites")))
      (:then_3
        (if (Variables|Features|GetShowFeatureSpritesAndTubes)
          (CallFunction|AddNiagaraSystemComponent (Math|Integer|Min(Integer) (- (+ (Variables|Default|GetNumberOfStreamLines) (Variables|Default|GetLinesOffset)) (+ (* _index (Variables|Default|GetMaxLinesPerComponent)) (Variables|Default|GetLinesOffset))) (Variables|Default|GetMaxLinesPerComponent)) (+ (* _index (Variables|Default|GetMaxLinesPerComponent)) (Variables|Default|GetLinesOffset)) "/DTCC_Visualization/Niagara/StreamlinesParticleSystem_SpritesAndTubes.StreamlinesParticleSystem_SpritesAndTubes")))
      (:then_4
        (if (Variables|Features|GetShowFeatureMovingMeshes)
          (CallFunction|AddNiagaraSystemComponent (Math|Integer|Min(Integer) (- (+ (Variables|Default|GetNumberOfStreamLines) (Variables|Default|GetLinesOffset)) (+ (* _index (Variables|Default|GetMaxLinesPerComponent)) (Variables|Default|GetLinesOffset))) (Variables|Default|GetMaxLinesPerComponent)) (+ (* _index (Variables|Default|GetMaxLinesPerComponent)) (Variables|Default|GetLinesOffset)) "/DTCC_Visualization/Niagara/StreamlinesParticleSystem_MovingMeshes.StreamlinesParticleSystem_MovingMeshes"))))))

(fn LoadandApplyData
  (bind _streamlinesegmentgenerator (Variables|Default|GetStreamlineSegmentGenerator))
  (bind _showfeaturestaticmesh (Variables|Features|GetShowFeatureStaticMesh))
  (bind _streamlinesegmentgenerator_2 (Variables|Default|GetStreamlineSegmentGenerator))
  (Utilities|FlowControl|Sequence
    (:then_0
      (CallFunction|PrepareData))
    (:then_1
      (CallFunction|InitateNiagraSystems))
    (:then_2
      (CallFunction|ApplyStreamlinesStyle))
    (:then_3
      (CallFunction|SetupDebug))
    (:then_4
      (Rendering|SetVisibility (Variables|Default|GetStaticStreamlines) _showfeaturestaticmesh true)
      (if _showfeaturestaticmesh
        (Variables|/Script/StreamlinesPlugin.StreamlineSegmentGenerator|SetStreamlinesDT _streamlinesegmentgenerator (.DataTable (Utilities|Struct|BreakLineDataTextureSource (Variables|Default|GetLineDataTextureSource))))
        (Variables|/Script/StreamlinesPlugin.StreamlineSegmentGenerator|SetAssignedCellSize _streamlinesegmentgenerator (Variables|Default|GetStaticMeshCellSize))
        (Variables|Default|SetStaticDrawCenterPosition (Class|KismetMathLibrary|VectorBoundedtoBox (Variables|Default|GetStaticDrawCenterPosition) (Variables|Default|GetDataPositionMin) (Variables|Default|GetDataPositionMax)))
        (Variables|/Script/StreamlinesPlugin.StreamlineSegmentGenerator|SetDrawCenterPosition _streamlinesegmentgenerator (Variables|Default|GetStaticDrawCenterPosition))
        (Variables|/Script/StreamlinesPlugin.StreamlineSegmentGenerator|SetStreamlineThickness _streamlinesegmentgenerator_2 (* (Variables|Default|GetLineWidth) 0.5))
        (Variables|/Script/StreamlinesPlugin.StreamlineSegmentGenerator|SetCapVertices _streamlinesegmentgenerator_2 (Variables|Default|GetStaticStreamlinesCapVertices))
        (Class|StreamlineSegmentGenerator|AssignStreamlinestoCells (Variables|Default|GetStreamlineSegmentGenerator))
        (CallFunction|GatherStaticStreamlines)))))

(fn GatherStaticStreamlines
  (bind _outactors (Actor|GetAllActorsOfClass "/Script/StreamlinesPlugin.Streamline"))
  (for _array_element _outactors
    (Transformation|AttachComponentToComponent _array_element (Variables|Default|GetStaticStreamlines) "None" "KeepRelative" "KeepRelative" "KeepRelative" true)))

(fn SetStaticDistanceCulling
  (for _array_element (Actor|GetAttachedActors true false)
    (bind _asstreamline (Utilities|Casting|CastToStreamline _array_element))
    (Class|PrimitiveComponent|SetCullDistance (Variables|/Script/StreamlinesPlugin.Streamline|GetVCProceduralMeshComponent _asstreamline) (Variables|Default|GetStaticCullDistance))))

(fn ToggleStaticVisible
  (for _array_element (Actor|GetAttachedActors true false)
    (bind _asstreamline (Utilities|Casting|CastToStreamline _array_element))
    (Rendering|ToggleVisibility (Variables|/Script/StreamlinesPlugin.Streamline|GetVCProceduralMeshComponent _asstreamline) false)))

(fn ToggleParticlesVisible
  (Rendering|ToggleVisibility (Variables|Default|GetParticleStreamlines) true))

(fn DestroyStaticStreamlines
  (bind _outactors (Actor|GetAllActorsOfClass "/Script/StreamlinesPlugin.Streamline"))
  (for _array_element _outactors
    (Actor|DestroyActor _array_element)))

(fn SpawnAllStaticStreamlinesinEditor
  (LocalVariables|SetPushedBurstCount (Variables|Spawning|GetSpawningBurstCount))
  (Variables|Spawning|SetSpawningBurstCount (Variables|Default|GetNumberOfStreamLines))
  (CallFunction|SpawnStreamlines)
  (Variables|Spawning|SetSpawningBurstCount (LocalVariables|GetPushedBurstCount)))

(fn AddNiagaraSystemComponent
  (params (NumberOfLines :type Integer) (LinesOffset :type Integer) (NiagraSystem :type Niagara%20System%20Object%20Reference))
  (bind _returnvalue (AddComponent|AddNiagaraComponent true))
  (Transformation|AttachComponentToComponent _returnvalue (Variables|Default|GetParticleStreamlines) "None" "KeepRelative" "KeepRelative" "KeepRelative" true)
  (Class|NiagaraComponent|SetAsset _returnvalue NiagraSystem true)
  (Utilities|Array|Add (Variables|Default|GetStreamlineSystems) _returnvalue)
  (CallFunction|SetupStreamlinesComponent _returnvalue NumberOfLines LinesOffset)
  (Development|PrintText (Utilities|Text|FormatText "Adding particle component ({type}, {n} lines, offset: {offs})" NiagraSystem NumberOfLines LinesOffset)))

(fn RedrawStaticMeshStreamlines
  (bind _linedatatexturesource (Variables|Default|GetLineDataTextureSource))
  (bind (_linetype _label _sourcepath _numlines _positionmin _positionmax _datamin _datamax _positiontexture _texturecombininglodivider _positiontexture_lo _datatexture _velocityspeedmin _velocityspeedmax) (Utilities|Struct|BreakLineDataTextureSource _linedatatexturesource))
  (if (Variables|Features|GetShowFeatureStaticMesh)
    (Class|StreamlineSegmentGenerator|DynamicStreamlineSpawn (Variables|Default|GetStreamlineSegmentGenerator))
    (CallFunction|GatherStaticStreamlines)
    (bind _outactors (Actor|GetAllActorsOfClass "/Script/StreamlinesPlugin.Streamline"))
    (for _array_element _outactors
      (Class|Streamline|PaintStreamline _array_element _velocityspeedmin _velocityspeedmax false)
      (Rendering|Material|SetMaterial (Variables|/Script/StreamlinesPlugin.Streamline|GetVCProceduralMeshComponent _array_element) 0 (Variables|Default|GetStaticStreamlineMaterial)))))