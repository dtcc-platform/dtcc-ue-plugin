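; Manager actor that controls the active colormap and value thresholds for data visualization materials.
; It bakes either a parametric colormap material or a colormap texture into a render target, at construction, at BeginPlay and roughly every second.
; Per-variable color and visibility ranges are scaled, normalized to the data domain and written to a material parameter collection, with show-all and threshold-only modes.
; Helper functions add variables, update ranges and map normalized values back to data units.
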(event Custom|BakeActiveColorMapTexture
  (bind _databakematerial (Variables|Default|GetDataBakeMaterial))
  ;[1 1 1] Bake selected colormap to active texture, used in active materials for current visualization
  (if (Variables|Default|GetUseParametricColormap)
    (Rendering|DrawMaterialtoRenderTarget "/DTCC_Visualization/RenderTargets/ActiveColorMap_RT.ActiveColorMap_RT" (Variables|BakingMaterials|GetParametricColormapMaterial))
    (else
      (Rendering|Material|SetTextureParameterValue _databakematerial "DataTexture" (Variables|Default|GetColorMapTexture))
      (Rendering|Material|SetMaterial (Variables|Default|GetCube) 0 _databakematerial)
      (Rendering|DrawMaterialtoRenderTarget "/DTCC_Visualization/RenderTargets/ActiveColorMap_RT.ActiveColorMap_RT" _databakematerial))))

(event Custom|Refresh)

(event Custom|ReBake
  (CallFunction|BakeActiveColorMapTexture))

(event EventTick
  (params (DeltaSeconds :type Float%20%28single-precision%29))
  (Utilities|FlowControl|Delay 1.0)
  (if true
    (CallFunction|ReBake)))

(event EventBeginPlay
  (CallFunction|ReBake)
  (VisualizationThresholds|ApplyDataVisualizationThresholds))

(fn ConstructionScript
  (Variables|VisualizationThresholds|SetInitialDataVisualizationRanges (Variables|VisualizationThresholds|GetDataVisualizationRanges))
  (bind _returnvalue (Rendering|Material|CreateDynamicMaterialInstance "/DTCC_Visualization/Materials/DataTexture_BakingMat.DataTexture_BakingMat" "None" "None" :!class /Script/Engine.KismetMaterialLibrary))
  (Variables|Default|SetDataBakeMaterial _returnvalue)
  (CallFunction|ReBake))

(fn GetCurrentDataVisualizationRanges
  (params (ApplyDataScale :type Boolean) (UseInitialRanges :type Boolean))
  (bind _datavisualizationranges (Variables|VisualizationThresholds|GetDataVisualizationRanges))
  (bind _initialdatavisualizationranges (Variables|VisualizationThresholds|GetInitialDataVisualizationRanges))
  (bind _datavariable (Variables|Default|GetDataVariable))
  (bind _returnvalue (select UseInitialRanges _initialdatavisualizationranges _datavisualizationranges))
  (bind (_value _returnvalue_2) (Utilities|Map|Find _returnvalue _datavariable))
  (return (select ApplyDataScale (VisualizationThresholds|ApplyDataScaleFactor _value) _value) _returnvalue_2 _datavariable ApplyDataScale))

(fn ApplyDataScaleFactor
  (params (VisualizationRanges :type Visualization%20Ranges%20Structure%20%28by%20ref%29))
  (bind (_datascalefactor _datadomain _colorscalerange _visibilityrange) (Utilities|Struct|BreakVisualizationRanges VisualizationRanges))
  (bind _returnvalue (Math|Conversions|ToFloat(Integer) _datascalefactor))
  (return (Utilities|Struct|MakeVisualizationRanges "1" "(X=0.000000,Y=0.000000)" (* _colorscalerange _returnvalue) (* _visibilityrange _returnvalue))))

(fn ApplyDataVisualizationThresholds
  (bind _showalldata (Variables|VisualizationThresholds|GetShowAllData))
  (bind _visualizationranges (VisualizationThresholds|GetCurrentDataVisualizationRangesNormalized false))
  (Rendering|Material|SetScalarParameterValue "/DTCC_Visualization/ParameterCollections/DataVisualizationThresholdParameters.DataVisualizationThresholdParameters" "ColormapMin" (.X (Math|Vector2D|BreakVector2D (.ColorScaleRange (Utilities|Struct|BreakVisualizationRanges _visualizationranges)))) :!class /Script/Engine.KismetMaterialLibrary)
  (Rendering|Material|SetScalarParameterValue "/DTCC_Visualization/ParameterCollections/DataVisualizationThresholdParameters.DataVisualizationThresholdParameters" "ColormapMax" (.Y (Math|Vector2D|BreakVector2D (.ColorScaleRange (Utilities|Struct|BreakVisualizationRanges _visualizationranges)))) :!class /Script/Engine.KismetMaterialLibrary)
  (Rendering|Material|SetScalarParameterValue "/DTCC_Visualization/ParameterCollections/DataVisualizationThresholdParameters.DataVisualizationThresholdParameters" "ShowMin" (Math|Float|SelectFloat -999999995904.0 (.X (Math|Vector2D|BreakVector2D (.VisibilityRange (Utilities|Struct|BreakVisualizationRanges _visualizationranges)))) _showalldata) :!class /Script/Engine.KismetMaterialLibrary)
  (Rendering|Material|SetScalarParameterValue "/DTCC_Visualization/ParameterCollections/DataVisualizationThresholdParameters.DataVisualizationThresholdParameters" "ShowMax" (Math|Float|SelectFloat 999999995904.0 (Math|Float|SelectFloat (* (.X (Math|Vector2D|BreakVector2D (.VisibilityRange (Utilities|Struct|BreakVisualizationRanges _visualizationranges)))) 1.2) (.Y (Math|Vector2D|BreakVector2D (.VisibilityRange (Utilities|Struct|BreakVisualizationRanges _visualizationranges)))) (Variables|VisualizationThresholds|GetShowOnlyThreshold)) _showalldata) :!class /Script/Engine.KismetMaterialLibrary)
  (bind _visualizationranges_2 (VisualizationThresholds|GetCurrentDataVisualizationRangesNormalized true))
  (Rendering|Material|SetScalarParameterValue "/DTCC_Visualization/ParameterCollections/DataVisualizationThresholdParameters.DataVisualizationThresholdParameters" "InitialShowMin" (.X (Math|Vector2D|BreakVector2D (.VisibilityRange (Utilities|Struct|BreakVisualizationRanges _visualizationranges_2)))) :!class /Script/Engine.KismetMaterialLibrary)
  (Rendering|Material|SetScalarParameterValue "/DTCC_Visualization/ParameterCollections/DataVisualizationThresholdParameters.DataVisualizationThresholdParameters" "ÏnitialShowMax" (Math|Float|SelectFloat (* (.X (Math|Vector2D|BreakVector2D (.VisibilityRange (Utilities|Struct|BreakVisualizationRanges _visualizationranges_2)))) 1.2) (.Y (Math|Vector2D|BreakVector2D (.VisibilityRange (Utilities|Struct|BreakVisualizationRanges _visualizationranges_2)))) (Variables|VisualizationThresholds|GetShowOnlyThreshold)) :!class /Script/Engine.KismetMaterialLibrary))

(fn GetCurrentDataVisualizationRangesNormalized
  (params (UseInitialRanges :type Boolean))
  (bind _visualizationranges (VisualizationThresholds|GetCurrentDataVisualizationRanges true UseInitialRanges))
  (bind _visualizationranges2 (VisualizationThresholds|ApplyDataScaleFactor _visualizationranges))
  (bind (_datascalefactor _datadomain _colorscalerange _visibilityrange) (Utilities|Struct|BreakVisualizationRanges _visualizationranges2))
  (bind (_x _y) (Math|Vector2D|BreakVector2D _datadomain))
  (bind _returnvalue (- _y _x))
  (return (Utilities|Struct|MakeVisualizationRanges (Utilities|String|ToString(Float) (/ 1.0 _returnvalue)) "(X=0.000000,Y=0.000000)" (/ (- _colorscalerange _x) _returnvalue) (/ (- _visibilityrange _x) _returnvalue))))

(fn SetDataVisualizationRangesChecked
  (params (VisualizationRanges :type Visualization%20Ranges%20Structure))
  (bind (_datascalefactor _datadomain _colorscalerange _visibilityrange) (Utilities|Struct|BreakVisualizationRanges VisualizationRanges))
  (bind _visualizationranges (VisualizationThresholds|GetCurrentDataVisualizationRanges false false))
  (bind _datascalefactor_2 (Utilities|Struct|BreakVisualizationRanges _visualizationranges))
  (bind _returnvalue (Math|Conversions|ToFloat(Integer) _datascalefactor))
  (bind _returnvalue_2 (Math|Conversions|ToFloat(Integer) _datascalefactor_2))
  (bind _returnvalue_3 (/ _returnvalue_2 _returnvalue))
  (Utilities|Map|Add (Variables|VisualizationThresholds|GetDataVisualizationRanges) (Variables|Default|GetDataVariable) (Utilities|Struct|MakeVisualizationRanges _datascalefactor_2 "(X=0.000000,Y=0.000000)" (/ _colorscalerange _returnvalue_3) (/ _visibilityrange _returnvalue_3))))

(fn MapNormalizedtoCurrentDataRange
  (params (VariableName :type String) (Value :type Float%20%28single-precision%29))
  (bind _datavisualizationranges (Variables|VisualizationThresholds|GetDataVisualizationRanges))
  (bind (_value _returnvalue) (Utilities|Map|Find _datavisualizationranges VariableName))
  (bind _datadomain (Utilities|Struct|BreakVisualizationRanges _value))
  (if _returnvalue
    (return (+ (* Value (- (.y _datadomain) (.x _datadomain))) (.x _datadomain)) true)
    (else
      (return 0.0 false))))

(fn AddScalarVariable
  (params (VariableName :type String) (MinValue :type Float%20%28single-precision%29) (MaxValue :type Float%20%28single-precision%29) (DataScaleFactor :type String))
  (bind _returnvalue (Math|Vector2D|MakeVector2D MinValue MaxValue))
  (Utilities|Map|Add (Variables|VisualizationThresholds|GetDataVisualizationRanges) VariableName (Utilities|Struct|MakeVisualizationRanges DataScaleFactor _returnvalue _returnvalue _returnvalue)))