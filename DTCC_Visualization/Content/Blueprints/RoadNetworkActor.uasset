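; RoadNetworkActor is an actor that configures a Niagara system with road network line data.
; Its construction script scans a data table of line data texture sources and keeps the first row whose type is RoadNetwork.
; It passes that row's data texture and min/max position bounds to Niagara, plus a sprite scale taken from the component's world X scale.
; The event graph holds no active logic.
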(event EventBeginPlay)

(event Collision|EventActorBeginOverlap
  (params (OtherActor :type Actor%20Object%20Reference)))

(event EventTick
  (params (DeltaSeconds :type Float%20%28single-precision%29)))

(fn ConstructionScript
  (bind _niagara (Variables|Default|GetNiagara))
  (Utilities|FlowControl|Sequence
    (:then_0
      (bind _outrownames (DataTable|GetDataTableRowNames "/Game/DTCC/DataImages/LineDataTextureSources_DT.LineDataTextureSources_DT"))
      (bind _array_element (Utilities|Array|ForEachLoopwithBreak _outrownames :!label _label)
        (:LoopBody
          (bind _returnvalue (Utilities|GetDataTableRow "/Game/DTCC/DataImages/LineDataTextureSources_DT.LineDataTextureSources_DT" _array_element)
            (:then
              (if (Utilities|Name|Equal(Name) (.LineType (Utilities|Struct|BreakLineDataTextureSource _returnvalue)) "RoadNetwork")
                (Variables|Default|SetLineDataTextureSource _returnvalue)
                (goto _label Break)))))))
    (:then_1
      (Effects|Components|ParticleSystem|SetVectorParameter _niagara "MinPosition" (.OutConvertedVector (Math|Conversions|ToVector(Float) (.PositionMin (Utilities|Struct|BreakLineDataTextureSource (Variables|Default|GetLineDataTextureSource))))))
      (Effects|Components|ParticleSystem|SetVectorParameter _niagara "MaxPosition" (.OutConvertedVector (Math|Conversions|ToVector(Float) (.PositionMax (Utilities|Struct|BreakLineDataTextureSource (Variables|Default|GetLineDataTextureSource))))))
      (Effects|Components|ParticleSystem|SetFloatParameter _niagara "SpriteScale" (.x (Transformation|GetWorldScale (Variables|Default|GetNiagara))))
      (Niagara|SetTextureObject _niagara "DataTexture" (.DataTexture (Utilities|Struct|BreakLineDataTextureSource (Variables|Default|GetLineDataTextureSource)))))))