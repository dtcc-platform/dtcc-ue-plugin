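; Construction-script builder that turns a data table of shapefile shapes into extruded procedural meshes, one section and shared material per row.
; A first pass finds the minimum point across all rows, which is subtracted to keep vertices local.
; Each shape's points are copied up by its height, with reversed triangles for the offset cap.
; Generated side triangles use duplicated vertices, intended to keep normals separate from the caps.
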(event EventBeginPlay)

(event Collision|EventActorBeginOverlap
  (params (OtherActor :type Actor%20Object%20Reference)))

(event EventTick
  (params (DeltaSeconds :type Float%20%28single-precision%29)))

(fn ConstructionScript
  (bind _newpoints (LocalVariables|GetNewPoints))
  (bind _proceduralmesh (Variables|Default|GetProceduralMesh))
  (bind _outrownames (DataTable|GetDataTableRowNames (Variables|Default|GetShapefileShapesDataTable)))
  (Utilities|FlowControl|Sequence
    (:then_0
      ;[1 1 1] Find min position, to offset all positions and make mesh more "local"
      (for _array_element _outrownames
        (bind _returnvalue (Utilities|GetDataTableRow (Variables|Default|GetShapefileShapesDataTable) _array_element)
          (:then
            (for _array_element_2 (.points (Utilities|Struct|BreakShapefileShape _returnvalue))
              (Utilities|FlowControl|Sequence
                (:then_0
                  ;;[1 1 1] Initiate
                  (Utilities|FlowControl|DoOnce false
                    (:Completed
                      (Variables|Default|SetMinPos _array_element_2))))
                (:then_1
                  (Variables|Default|SetMinPos (Math|Vector|VectorComponentMin _array_element_2 (Variables|Default|GetMinPos))))))))))
    (:then_1
      (for (_array_element_3 _array_index) _outrownames
        (bind _returnvalue_2 (Utilities|GetDataTableRow (Variables|Default|GetShapefileShapesDataTable) _array_element_3)
          (:then
            (Utilities|FlowControl|Sequence
              (:then_0
                ;[1 1 1] Setup vertices
                (Utilities|FlowControl|Sequence
                  (:then_0
                    ;[1 1 1] Translate to "local" (subtract min position)
                    (Utilities|Array|Clear (LocalVariables|GetNewPoints))
                    (for _array_element_4 (.points (Utilities|Struct|BreakShapefileShape _returnvalue_2))
                      (Utilities|Array|Add (LocalVariables|GetNewPoints) (- _array_element_4 (Variables|Default|GetMinPos)))))
                  (:then_1
                    ;[1 1 1] Add offset height points
                    (bind _output_get (LocalVariables|SetTmpPoints (LocalVariables|GetNewPoints)))
                    (for _array_element_5 _output_get
                      (Utilities|Array|Add (LocalVariables|GetNewPoints) (+ _array_element_5 (Math|Vector|MakeVector 0.0 0.0 (.height (Utilities|Struct|BreakShapefileShape _returnvalue_2)))))))
                  (:then_2
                    ;[1 1 1] Duplicate for sides (for normals)
                    (bind _output_get_2 (LocalVariables|SetTmpPoints (LocalVariables|GetNewPoints)))
                    (for _array_element_6 _output_get_2
                      ;;[1 1 1] Add twice for normals
                      (Utilities|Array|Add _newpoints _array_element_6)
                      (Utilities|Array|Add _newpoints _array_element_6)))))
              (:then_1
                ;[1 1 1] Setup triangles
                (Utilities|FlowControl|Sequence
                  (:then_0
                    ;[1 1 1] Original triangles
                    (LocalVariables|SetNewTriangles (.triangles (Utilities|Struct|BreakShapefileShape _returnvalue_2)))
                    (Variables|Default|SetOriginalNumberOfPoints (Utilities|Array|Length (.points (Utilities|Struct|BreakShapefileShape _returnvalue_2)))))
                  (:then_1
                    ;[1 1 1] Height offset triangles
                    (bind _arrayelement (Utilities|Array|ReverseforEachLoop (.triangles (Utilities|Struct|BreakShapefileShape _returnvalue_2)))
                      (:LoopBody
                        (Utilities|Array|Add (LocalVariables|GetNewTriangles) (+ (Variables|Default|GetOriginalNumberOfPoints) _arrayelement)))))
                  (:then_2
                    ;[1 1 1] Add sides
                    (for _index (range 0 (- (Variables|Default|GetOriginalNumberOfPoints) 1))
                      (Utilities|FlowControl|Sequence
                        (:then_0
                          (Utilities|FlowControl|Sequence
                            (:then_0
                              (Utilities|Array|Add (LocalVariables|GetNewTriangles) (+ (+ (* _index 2) (* (Variables|Default|GetOriginalNumberOfPoints) 2)) 1)))
                            (:then_1
                              (Utilities|Array|Add (LocalVariables|GetNewTriangles) (+ (+ (* _index 2) (* (Variables|Default|GetOriginalNumberOfPoints) 2)) 2)))
                            (:then_2
                              (Utilities|Array|Add (LocalVariables|GetNewTriangles) (+ (+ (+ (* _index 2) (* (Variables|Default|GetOriginalNumberOfPoints) 2)) 1) (* (Variables|Default|GetOriginalNumberOfPoints) 2))))))
                        (:then_1
                          (Utilities|FlowControl|Sequence
                            (:then_0
                              (Utilities|Array|Add (LocalVariables|GetNewTriangles) (+ (+ (* _index 2) (* (Variables|Default|GetOriginalNumberOfPoints) 2)) 2)))
                            (:then_1
                              (Utilities|Array|Add (LocalVariables|GetNewTriangles) (+ (+ (+ (+ (* _index 2) (* (Variables|Default|GetOriginalNumberOfPoints) 2)) 1) (* (Variables|Default|GetOriginalNumberOfPoints) 2)) 1)))
                            (:then_2
                              (Utilities|Array|Add (LocalVariables|GetNewTriangles) (+ (+ (+ (* _index 2) (* (Variables|Default|GetOriginalNumberOfPoints) 2)) 1) (* (Variables|Default|GetOriginalNumberOfPoints) 2)))))))))))
              (:then_2
                (Class|ProceduralMeshComponent|CreateMeshSectionLinearColor _proceduralmesh _array_index (LocalVariables|GetNewPoints) (LocalVariables|GetNewTriangles) 0 0 0 0 0 0 0 false)
                (Rendering|Material|SetMaterial _proceduralmesh _array_index "/Game/InfravisTest/ShapeMat.ShapeMat")))))))))