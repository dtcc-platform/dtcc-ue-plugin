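; Manager actor for volumetric data visualization that loads scenario and variable textures from a data table and bakes them for rendering.
; Dynamic materials draw colormap, colored, normalized, mask and velocity render targets, optionally rebaking on a delayed Tick.
; Material parameter collections receive placement and range-normalized color and visibility thresholds.
; GetDataAtPoint converts world positions to UVs in an 8x8 slice atlas, reading back values in data units.
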(event Custom|BakeActiveColorMapTexture
  (bind _databakematerial (Variables|BakingMaterials|GetDataBakeMaterial))
  ;[1 1 1] Bake selected colormap to active texture, used in active materials for current visualization
  (if (Variables|Default|GetUseParametricColormap)
    (Rendering|DrawMaterialtoRenderTarget "/DTCC_Visualization/RenderTargets/ActiveColorMap_RT.ActiveColorMap_RT" (Variables|BakingMaterials|GetParametricColormapMaterial))
    (else
      (Rendering|Material|SetTextureParameterValue _databakematerial "DataTexture" (Variables|Default|GetColorMapTexture))
      (Rendering|DrawMaterialtoRenderTarget "/DTCC_Visualization/RenderTargets/ActiveColorMap_RT.ActiveColorMap_RT" _databakematerial))))

(event Custom|BakeActiveDataTexture
  (bind _coloreddatabakingmaterial (Variables|BakingMaterials|GetColoredDataBakingMaterial))
  (bind _greydatabakingmaterial (Variables|BakingMaterials|GetGreyDataBakingMaterial))
  (bind _databakematerial (Variables|BakingMaterials|GetDataBakeMaterial))
  ;[1 1 1] Bake selected data to active texture, used in active materials for current visualization
  (Rendering|Material|SetTextureParameterValue _coloreddatabakingmaterial "DataTexture" (Variables|Default|GetSelectedDataTexture))
  (Rendering|DrawMaterialtoRenderTarget "/DTCC_Visualization/RenderTargets/ActiveDataClampedColorTexture_RT.ActiveDataClampedColorTexture_RT" _coloreddatabakingmaterial)
  (Rendering|Material|SetTextureParameterValue _databakematerial "DataTexture" (Variables|Default|GetSelectedDataTexture))
  (Rendering|DrawMaterialtoRenderTarget "/DTCC_Visualization/RenderTargets/ActiveDataNormalizedTexture_RT.ActiveDataNormalizedTexture_RT" _databakematerial)
  (if (Variables|VisualizationThresholds|GetShowAllData)
    _
    (else
      _))
  (Rendering|Material|SetTextureParameterValue _greydatabakingmaterial "DataTexture" (Variables|Default|GetSelectedDataTexture))
  (Rendering|DrawMaterialtoRenderTarget "/DTCC_Visualization/RenderTargets/ActiveDataMaskTexture_RT.ActiveDataMaskTexture_RT" _greydatabakingmaterial))

(event Custom|Refresh
  (CallFunction|LoadScenarioDataTexture (Variables|Default|GetScenarioLabel)))

(event Custom|ReBake
  (CallFunction|BakeActiveColorMapTexture)
  (CallFunction|BakeActiveDataTexture)
  (Baking|BakeVelocityTexture))

(event Custom|TestGetDataAtPoint
  (CallFunction|GetDataatPoint (Transformation|GetWorldLocation (Variables|Default|GetDefaultSceneRoot))))

(event EventTick
  (params (DeltaSeconds :type Float%20%28single-precision%29))
  (Utilities|FlowControl|Delay 1.0)
  (if (Variables|Default|GetAutoRefreshDataTextures)
    (CallFunction|ReBake)))

(event EventBeginPlay
  (CallFunction|PushPositionParameterstoCollection)
  (CallFunction|ReBake)
  (VisualizationThresholds|ApplyDataVisualizationThresholds))

(fn ConstructionScript
  (bind _benabledebug (Variables|Default|GetbEnableDebug))
  (CallFunction|TestGetDataatPoint)
  (bind _returnvalue (Rendering|Material|CreateDynamicMaterialInstance "/DTCC_Visualization/Materials/DataTexture_BakingMat.DataTexture_BakingMat" "None" "None" :!class /Script/Engine.KismetMaterialLibrary))
  (Variables|BakingMaterials|SetDataBakeMaterial _returnvalue)
  (bind _returnvalue_2 (Rendering|Material|CreateDynamicMaterialInstance "/DTCC_Visualization/Materials/ColorMappedClampedDataTexture_BakingMat.ColorMappedClampedDataTexture_BakingMat" "None" "None" :!class /Script/Engine.KismetMaterialLibrary))
  (Variables|BakingMaterials|SetColoredDataBakingMaterial _returnvalue_2)
  (bind _returnvalue_3 (Rendering|Material|CreateDynamicMaterialInstance "/DTCC_Visualization/Materials/DataTextureMasked_BakingMat.DataTextureMasked_BakingMat" "None" "None" :!class /Script/Engine.KismetMaterialLibrary))
  (Variables|BakingMaterials|SetGreyDataBakingMaterial _returnvalue_3)
  (bind _returnvalue_4 (Rendering|Material|CreateDynamicMaterialInstance "/DTCC_Visualization/Materials/DataTextureVelocity_BakingMat.DataTextureVelocity_BakingMat" "None" "None" :!class /Script/Engine.KismetMaterialLibrary))
  (Variables|BakingMaterials|SetVelocityDataBakeMaterial _returnvalue_4)
  (CallFunction|LoadScenarioDataTexture (Variables|Default|GetScenarioLabel))
  (Variables|VisualizationThresholds|SetInitialDataVisualizationRanges (Variables|VisualizationThresholds|GetDataVisualizationRanges))
  (CallFunction|PushPositionParameterstoCollection)
  (CallFunction|ReBake)
  (Rendering|SetVisibility (Variables|Default|GetDebugging) _benabledebug true)
  (if _benabledebug
    (Rendering|Material|SetMaterial (Variables|Default|GetCube) 0 (Variables|BakingMaterials|GetDataBakeMaterial))
    (Rendering|Material|SetMaterial (Variables|Default|GetCube1) 0 (Variables|BakingMaterials|GetColoredDataBakingMaterial))
    (Rendering|Material|SetMaterial (Variables|Default|GetCube2) 0 (Variables|BakingMaterials|GetGreyDataBakingMaterial))
    (Rendering|Material|SetMaterial (Variables|Default|GetCube3) 0 (Variables|BakingMaterials|GetVelocityDataBakeMaterial))))

(fn GetDataatPoint
  (params (WorldLocation :type Vector))
  (bind _returnvalue (Rendering|Material|GetVectorParameterValue "/DTCC_Visualization/ParameterCollections/VolumetricDataPositioningParameters.VolumetricDataPositioningParameters" "PositionOffset" :!class /Script/Engine.KismetMaterialLibrary))
  (bind _returnvalue_2 (Rendering|Material|GetVectorParameterValue "/DTCC_Visualization/ParameterCollections/VolumetricDataPositioningParameters.VolumetricDataPositioningParameters" "Scale" :!class /Script/Engine.KismetMaterialLibrary))
  (bind _returnvalue_3 (Rendering|Material|GetScalarParameterValue "/DTCC_Visualization/ParameterCollections/VolumetricDataPositioningParameters.VolumetricDataPositioningParameters" "Rotation" :!class /Script/Engine.KismetMaterialLibrary))
  (bind _uv (CallFunction|CalculateUVfromXYZ (+ (Math|Vector|RotateVectorAroundAxis (* (* (- WorldLocation (Math|Conversions|ToVector(LinearColor) _returnvalue)) "1.000000,-1.000000,1.000000") (/ "0.010000,0.010000,0.010000" (Math|Conversions|ToVector(LinearColor) _returnvalue_2))) (* _returnvalue_3 -1.0) "0, 0,1.000000") "0.500000,0.500000,0.000000")))
  (bind _returnvalue_4 (Rendering|ReadRenderTargetRawUV "/DTCC_Visualization/RenderTargets/ActiveDataNormalizedTexture_RT.ActiveDataNormalizedTexture_RT" (.X (Math|Vector2D|BreakVector2D _uv)) (.Y (Math|Vector2D|BreakVector2D _uv))))
  (bind (_rangedvalue _isvalid) (CallFunction|MapNormalizedtoCurrentDataRange (.R (Utilities|Struct|BreakLinearColor _returnvalue_4))))
  (return _rangedvalue (+ (Math|Vector|RotateVectorAroundAxis (* (* (- WorldLocation (Math|Conversions|ToVector(LinearColor) _returnvalue)) "1.000000,-1.000000,1.000000") (/ "0.010000,0.010000,0.010000" (Math|Conversions|ToVector(LinearColor) _returnvalue_2))) (* _returnvalue_3 -1.0) "0, 0,1.000000") "0.500000,0.500000,0.000000") _uv _isvalid))

(fn LoadScenarioDataTexture
  (params (ScenarioLabel :type String))
  (bind _velocityvariable (Variables|Default|GetVelocityVariable))
  (bind _velocitydatabakematerial (Variables|BakingMaterials|GetVelocityDataBakeMaterial))
  (bind _datatexturesource (CallFunction|GetCurrentDataTextureSource _velocityvariable))
  (bind (_sourcefile _scenariolabel _variablename _dataminvalue _datamaxvalue _dataunit _datatexture) (Utilities|Struct|BreakDataTextureSource _datatexturesource))
  (bind _outconvertedvector (Math|Conversions|ToVector(Float) _dataminvalue))
  (if (Utilities|Enum|NotEqual(Enum) ScenarioLabel "")
    (Variables|Default|SetScenarioLabel ScenarioLabel))
  (bind _datatexture_2 (CallFunction|GetCurrentDataTexture))
  (Variables|Default|SetSelectedDataTexture _datatexture_2)
  (VisualizationThresholds|ApplyDataVisualizationThresholds)
  (CallFunction|ReBake)
  (if (Utilities|Enum|NotEqual(Enum) (Variables|Default|GetVelocityVariable) "")
    (bind _output_get (Variables|Default|SetSelectedVelocityTexture _datatexture))
    (Rendering|Material|SetTextureParameterValue _velocitydatabakematerial "DataTexture" _output_get)
    (Rendering|Material|SetVectorParameterValue _velocitydatabakematerial "VelocityOffset" (Math|Conversions|ToLinearColor(Vector) _outconvertedvector) :!class /Script/Engine.MaterialInstanceDynamic)
    (Rendering|Material|SetVectorParameterValue _velocitydatabakematerial "VelocityScale" (Math|Conversions|ToLinearColor(Vector) (- (.OutConvertedVector (Math|Conversions|ToVector(Float) _datamaxvalue)) _outconvertedvector)) :!class /Script/Engine.MaterialInstanceDynamic)
    (Baking|BakeVelocityTexture)))

(fn GetCurrentDataTextureSource
  (params (DataVariable :type String))
  (bind _scenariolabel (Variables|Default|GetScenarioLabel))
  (bind (_datatexturesource _isvalid) (CallFunction|GetDataTextureSource DataVariable _scenariolabel))
  (return _datatexturesource _isvalid))

(fn GetCurrentDataVisualizationRanges
  (params (ApplyDataScale :type Boolean) (UseInitialRanges :type Boolean))
  (bind _datavisualizationranges (Variables|VisualizationThresholds|GetDataVisualizationRanges))
  (bind _initialdatavisualizationranges (Variables|VisualizationThresholds|GetInitialDataVisualizationRanges))
  (bind _datavariable (Variables|Default|GetDataVariable))
  (bind _returnvalue (select UseInitialRanges _initialdatavisualizationranges _datavisualizationranges))
  (bind (_value _returnvalue_2) (Utilities|Map|Find _returnvalue _datavariable))
  (return (select ApplyDataScale (VisualizationThresholds|ApplyDataScaleFactor _value) _value) _returnvalue_2 _datavariable ApplyDataScale))

(fn ApplyDataScaleFactor
  (params (VisualizationRanges :type Visualization%20Ranges%20Structure%20%28by%20ref%29))
  (bind (_datascalefactor _datadomain _colorscalerange _visibilityrange) (Utilities|Struct|BreakVisualizationRanges VisualizationRanges))
  (bind _returnvalue (Math|Conversions|ToFloat(Integer) _datascalefactor))
  (return (Utilities|Struct|MakeVisualizationRanges "1" "(X=0.000000,Y=0.000000)" (* _colorscalerange _returnvalue) (* _visibilityrange _returnvalue))))

(fn ApplyDataVisualizationThresholds
  (bind _showalldata (Variables|VisualizationThresholds|GetShowAllData))
  (bind _visualizationranges (VisualizationThresholds|GetCurrentDataVisualizationRangesNormalized false))
  (Rendering|Material|SetScalarParameterValue "/DTCC_Visualization/ParameterCollections/DataVisualizationThresholdParameters.DataVisualizationThresholdParameters" "ColormapMin" (.X (Math|Vector2D|BreakVector2D (.ColorScaleRange (Utilities|Struct|BreakVisualizationRanges _visualizationranges)))) :!class /Script/Engine.KismetMaterialLibrary)
  (Rendering|Material|SetScalarParameterValue "/DTCC_Visualization/ParameterCollections/DataVisualizationThresholdParameters.DataVisualizationThresholdParameters" "ColormapMax" (.Y (Math|Vector2D|BreakVector2D (.ColorScaleRange (Utilities|Struct|BreakVisualizationRanges _visualizationranges)))) :!class /Script/Engine.KismetMaterialLibrary)
  (Rendering|Material|SetScalarParameterValue "/DTCC_Visualization/ParameterCollections/DataVisualizationThresholdParameters.DataVisualizationThresholdParameters" "ShowMin" (Math|Float|SelectFloat -999999995904.0 (.X (Math|Vector2D|BreakVector2D (.VisibilityRange (Utilities|Struct|BreakVisualizationRanges _visualizationranges)))) _showalldata) :!class /Script/Engine.KismetMaterialLibrary)
  (Rendering|Material|SetScalarParameterValue "/DTCC_Visualization/ParameterCollections/DataVisualizationThresholdParameters.DataVisualizationThresholdParameters" "ShowMax" (Math|Float|SelectFloat 999999995904.0 (Math|Float|SelectFloat (* (.X (Math|Vector2D|BreakVector2D (.VisibilityRange (Utilities|Struct|BreakVisualizationRanges _visualizationranges)))) 1.2) (.Y (Math|Vector2D|BreakVector2D (.VisibilityRange (Utilities|Struct|BreakVisualizationRanges _visualizationranges)))) (Variables|VisualizationThresholds|GetShowOnlyThreshold)) _showalldata) :!class /Script/Engine.KismetMaterialLibrary)
  (bind _visualizationranges_2 (VisualizationThresholds|GetCurrentDataVisualizationRangesNormalized true))
  (Rendering|Material|SetScalarParameterValue "/DTCC_Visualization/ParameterCollections/DataVisualizationThresholdParameters.DataVisualizationThresholdParameters" "InitialShowMin" (.X (Math|Vector2D|BreakVector2D (.VisibilityRange (Utilities|Struct|BreakVisualizationRanges _visualizationranges_2)))) :!class /Script/Engine.KismetMaterialLibrary)
  (Rendering|Material|SetScalarParameterValue "/DTCC_Visualization/ParameterCollections/DataVisualizationThresholdParameters.DataVisualizationThresholdParameters" "ÏnitialShowMax" (Math|Float|SelectFloat (* (.X (Math|Vector2D|BreakVector2D (.VisibilityRange (Utilities|Struct|BreakVisualizationRanges _visualizationranges_2)))) 1.2) (.Y (Math|Vector2D|BreakVector2D (.VisibilityRange (Utilities|Struct|BreakVisualizationRanges _visualizationranges_2)))) (Variables|VisualizationThresholds|GetShowOnlyThreshold)) :!class /Script/Engine.KismetMaterialLibrary))

(fn GetCurrentDataVisualizationRangesNormalized
  (params (UseInitialRanges :type Boolean))
  (bind _visualizationranges (VisualizationThresholds|GetCurrentDataVisualizationRanges true UseInitialRanges))
  (bind _datatexturesource (CallFunction|GetCurrentDataTextureSource))
  (bind (_sourcefile _scenariolabel _variablename _dataminvalue _datamaxvalue) (Utilities|Struct|BreakDataTextureSource _datatexturesource))
  (bind _visualizationranges2 (VisualizationThresholds|ApplyDataScaleFactor _visualizationranges))
  (bind (_datascalefactor _datadomain _colorscalerange _visibilityrange) (Utilities|Struct|BreakVisualizationRanges _visualizationranges2))
  (bind _returnvalue (Math|Conversions|ToFloat(Integer) _dataminvalue))
  (bind _returnvalue_2 (Math|Conversions|ToFloat(Integer) _datamaxvalue))
  (bind _returnvalue_3 (- _returnvalue_2 _returnvalue))
  (return (Utilities|Struct|MakeVisualizationRanges (Utilities|String|ToString(Float) (/ 1.0 _returnvalue_3)) "(X=0.000000,Y=0.000000)" (/ (- _colorscalerange _returnvalue) _returnvalue_3) (/ (- _visibilityrange _returnvalue) _returnvalue_3))))

(fn SetDataVisualizationRangesChecked
  (params (VisualizationRanges :type Visualization%20Ranges%20Structure))
  (bind (_datascalefactor _datadomain _colorscalerange _visibilityrange) (Utilities|Struct|BreakVisualizationRanges VisualizationRanges))
  (bind _visualizationranges (VisualizationThresholds|GetCurrentDataVisualizationRanges false false))
  (bind _datascalefactor_2 (Utilities|Struct|BreakVisualizationRanges _visualizationranges))
  (bind _returnvalue (Math|Conversions|ToFloat(Integer) _datascalefactor))
  (bind _returnvalue_2 (Math|Conversions|ToFloat(Integer) _datascalefactor_2))
  (bind _returnvalue_3 (/ _returnvalue_2 _returnvalue))
  (Utilities|Map|Add (Variables|VisualizationThresholds|GetDataVisualizationRanges) (Variables|Default|GetDataVariable) (Utilities|Struct|MakeVisualizationRanges _datascalefactor_2 "(X=0.000000,Y=0.000000)" (/ _colorscalerange _returnvalue_3) (/ _visibilityrange _returnvalue_3))))

(fn MapNormalizedtoCurrentDataRange
  (params (Value :type Float%20%28double-precision%29))
  (bind (_datatexturesource _isvalid) (CallFunction|GetCurrentDataTextureSource))
  (bind (_sourcefile _scenariolabel _variablename _dataminvalue _datamaxvalue) (Utilities|Struct|BreakDataTextureSource _datatexturesource))
  (bind _returnvalue (Math|Conversions|ToFloat(Integer) _dataminvalue))
  (return (+ (* Value (- (Math|Conversions|ToFloat(Integer) _datamaxvalue) _returnvalue)) _returnvalue) _isvalid))

(fn GetCurrentDataTexture
  (params (DataVariable :type String))
  (bind (_datatexturesource _isvalid) (CallFunction|GetCurrentDataTextureSource DataVariable))
  (if _isvalid
    (return (.DataTexture (Utilities|Struct|BreakDataTextureSource _datatexturesource)))
    (else
      (Development|PrintString "Data texture source NOT FOUND in data table!" true true "(R=1.000000,G=0.493793,B=0.091597,A=1.000000)")
      (return 0))))

(fn CalculateUVfromXYZ
  (params (InVec :type Vector))
  (bind (_x _y _z) (Math|Vector|BreakVector InVec))
  (bind _returnvalue (* _z 64.0))
  (bind _returnvalue_2 (/ _returnvalue 8.0))
  (return (+ (* (Math|Vector2D|MakeVector2D _x _y) 0.125) (* (Math|Vector2D|MakeVector2D (Math|Conversions|ToFloat(Integer) (Math|Float|Floor _returnvalue_2)) (Math|Conversions|ToFloat(Integer) (Math|Float|Floor (* (Math|Float|Fraction _returnvalue_2) 8.0)))) 0.125))))

(fn BakeVelocityTexture
  (Rendering|DrawMaterialtoRenderTarget "/DTCC_Visualization/RenderTargets/ActiveDataVelocityTexture_RT.ActiveDataVelocityTexture_RT" (Variables|BakingMaterials|GetVelocityDataBakeMaterial)))

(fn GetDataTextureSource
  (params (DataVariable :type String) (ScenarioLabel :type String))
  (bind _returnvalue (Utilities|Enum|Equal(Enum) DataVariable ""))
  (bind _returnvalue_2 (select _returnvalue (Variables|Default|GetDataVariable) DataVariable))
  (bind _returnvalue_3 (Utilities|GetDataTableRow (Variables|Default|GetDataTextureSourcesTable) (Utilities|String|StringToName (Utilities|String|Append ScenarioLabel _returnvalue_2)))
    (:then
      (return _returnvalue_3 true))
    (:RowNotFound
      (return (Utilities|Struct|MakeDataTextureSource "Data Source Not Found!" (Utilities|String|StringToName ScenarioLabel) (Utilities|String|StringToName _returnvalue_2) "0" "1") false))))

(fn PushPositionParameterstoCollection
  (Rendering|Material|SetVectorParameterValue "/DTCC_Visualization/ParameterCollections/VolumetricDataPositioningParameters.VolumetricDataPositioningParameters" "PositionOffset" (Math|Conversions|ToLinearColor(Vector) (Variables|Default|GetDataPositionOffset)) :!class /Script/Engine.KismetMaterialLibrary)
  (Rendering|Material|SetVectorParameterValue "/DTCC_Visualization/ParameterCollections/VolumetricDataPositioningParameters.VolumetricDataPositioningParameters" "Scale" (Math|Conversions|ToLinearColor(Vector) (Variables|Default|GetDataScale)) :!class /Script/Engine.KismetMaterialLibrary)
  (Rendering|Material|SetScalarParameterValue "/DTCC_Visualization/ParameterCollections/VolumetricDataPositioningParameters.VolumetricDataPositioningParameters" "DataTextureColumns" (Math|Conversions|ToFloat(Integer) (Variables|Default|GetDataTextureColumns)) :!class /Script/Engine.KismetMaterialLibrary)
  (Rendering|Material|SetScalarParameterValue "/DTCC_Visualization/ParameterCollections/VolumetricDataPositioningParameters.VolumetricDataPositioningParameters" "DataTextureRows" (Math|Conversions|ToFloat(Integer) (Variables|Default|GetDataTextureRows)) :!class /Script/Engine.KismetMaterialLibrary))